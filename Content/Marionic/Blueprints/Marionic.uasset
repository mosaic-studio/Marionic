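; Marionic is a 2D flipbook player character with axis movement, jumping by key or touch, a points counter and a HUD widget.
; A States variable selects the flipbook, and Tick flips facing from X velocity and runs a debug downward trace while airborne.
; HealthSystem, also triggered by a test F key, disables input and either sets Dead or applies knockback force.
; Landing after a hit restores input following a short delay.
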(event `Health System`
  (params (vida :type "Float (double-precision)"))
  ;[1 1 1] Health System
  (set `self.isHit` true)
  (`self.DisableInput` (`GameplayStatics.GetPlayerController` 0))
  (bind _output_get (set `self.vida` (- (`self.vida`) vida)))
  (if (<= _output_get 0.0)
    (set `self.states` "NewEnumerator5")
    (`self.DisableInput` (`GameplayStatics.GetPlayerController` 0))
    (else
      (set `self.states` "NewEnumerator6")
      (`CharacterMovementComponent.AddForce` (`self.CharacterMovement`) (`KismetMathLibrary.MakeVector` (* (`self.Facing`) (`self.Knockback`)) 0.0 700000.0)))))

(event `Key|F`
  (params (Key :type "Key Structure" :default "AnyKey"))
  (:`Pressed`
    (`self.Health System` 0.25)))

(event `self.ReceiveBeginPlay`
  ;[1 1 1] Inicialização
  (`|ExecutionSequence`
    (:`then_0`
      (`ActorComponent.SetIsReplicated` (`self.Sprite`) true))
    (:`then_1`
      (bind _returnvalue (`|CreateWidget` "/Game/Marionic/Blueprints/HUD_Marionic.HUD_Marionic_C" (`GameplayStatics.GetPlayerController` 0)))
      (bind _output_get (set `self.pontosTexto` _returnvalue))
      (`UserWidget.AddToViewport` _output_get 0))))

(event `Points System`
  (params (valor :type Integer))
  (set `self.pontos` (+ valor (`self.pontos`))))

(event `UpdateAnimation`
  ;[1 1 1] Handle Animation
  (switch `/Game/Marionic/Enum/states_player` (`self.states`)
    (:`NewEnumerator0`
      (`PaperFlipbookComponent.SetFlipbook` (`self.Sprite`) (select `bool` (> (`KismetMathLibrary.VSize` (`self.GetVelocity`)) 0.0) :`false` "/Game/Marionic/Sprites/Player1/p1_idle.p1_idle" :`true` "/Game/Marionic/Sprites/Player1/p1_walk.p1_walk" :!type "PaperFlipbook Object Reference")))
    (:`NewEnumerator1`
      (`PaperFlipbookComponent.SetFlipbook` (`self.Sprite`) "/Game/Marionic/Sprites/Player1/p1_jumping.p1_jumping"))
    (:`NewEnumerator6`
      (`PaperFlipbookComponent.SetFlipbook` (`self.Sprite`) "/Game/Marionic/Sprites/Player1/p1_hit.p1_hit"))))

(event `self.ReceiveTick`
  (params (DeltaSeconds :type "Float (single-precision)"))
  (bind _returnvalue (`self.K2_GetActorLocation` self))
  ;[1 1 1] Tick - Updates animation
  (`|ExecutionSequence`
    (:`then_0`
      (if (not (`NavMovementComponent.IsMovingOnGround` (`self.CharacterMovement`)))
        (bind _outhit (`KismetSystemLibrary.LineTraceSingle` :`Start` _returnvalue :`End` (+ _returnvalue (* (`self.GetActorUpVector` self) -110.0)) :`TraceChannel` "TraceTypeQuery1" :`DrawDebugType` "Persistent"))
        (`KismetSystemLibrary.PrintString` (`KismetSystemLibrary.GetDisplayName` (`.HitActor` (`GameplayStatics.BreakHitResult` _outhit))))))
    (:`then_1`
      (`self.UpdateAnimation`)
      (`/Engine/EditorBlueprintResources/StandardMacros.CompareFloat` (.x (`MovementComponent.Velocity` (`self.GetMovementComponent`)))
        (:`>`
          (`Controller.SetControlRotation` (`self.GetController`) (`KismetMathLibrary.MakeRotator` 0.0 0.0 0.0))
          (set `self.Facing` 1))
        (:`<`
          (`Controller.SetControlRotation` (`self.GetController`) (`KismetMathLibrary.MakeRotator` 0.0 0.0 180.0))
          (set `self.Facing` -1))))))

(event `InputAxis|MoveRight`
  (params (AxisValue :type "Float (single-precision)"))
  (bind _velocidade (`self.velocidade`))
  ;[1 1 1] Handle movement
  (`self.AddMovementInput` (1.0 0.0 0.0) (* (/ AxisValue (`self.velocidade`)) (`KismetMathLibrary.FClamp` (* (stale `InputAxis|Sprint` AxisValue) _velocidade) (`self.velociCaminhando`) _velocidade))))

(event `InputAxis|Sprint`
  (params (AxisValue :type "Float (single-precision)"))
  ;[1 1 1] Handle movement
)

(event `InputAction|Jump`
  (params (Key :type "Key Structure" :default "AnyKey"))
  ;[1 1 1] Handle Jump
  (:`Pressed`
    (`self.Jump` :!label _label)
    (set `self.states` "NewEnumerator1"))
  (:`Released`
    (`self.StopJumping` :!label _label_2)))

(event `InputTouch`
  (params (Location :type "Vector Structure") (FingerIndex :type "ETouchIndex Enum"))
  ;[1 1 1] Handle Jump
  (:`Pressed`
    (goto _label))
  (:`Released`
    (goto _label_2)))

(event `self.OnLanded`
  (params (Hit :type "HitResult Structure (by ref)"))
  ;[1 1 1] Evento Ao Aterrissar
  (if (`self.isHit`)
    (set `self.states` "NewEnumerator7")
    (`self.UpdateAnimation`)
    (`KismetSystemLibrary.Delay` 0.5)
    (set `self.isHit` false)
    (set `self.states` "NewEnumerator0")
    (`self.UpdateAnimation`)
    (`self.EnableInput` (`GameplayStatics.GetPlayerController` 0))
    (else
      (set `self.states` "NewEnumerator0")
      (`self.UpdateAnimation`))))

(fn `UserConstructionScript`)