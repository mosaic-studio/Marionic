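; PawnFly is a flying enemy in the Marionic game that damages Marionic on overlap with its Box.
; A timeline lerps it between the Point0 and Point1 actors, mirroring the flipbook's X scale near each end.
; KillFly calls Stop on that timeline, whose Finished output shows the dead flipbook, deactivates the Box and destroys the actor after a short delay.
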(event `self.ReceiveBeginPlay`)

(event `self.ReceiveActorBeginOverlap`
  (params (OtherActor :type "Actor Object Reference")))

(event `self.ReceiveTick`
  (params (DeltaSeconds :type "Float (single-precision)")))

(event `Kill Fly`
  (bind _paperflipbook (`self.PaperFlipbook`))
  (bind (_direction _alphavalue) (`Timeline|Linha do Tempo_0` :!via `Stop`)
    (:`Update`
      (`self.K2_SetActorLocation` self (`KismetMathLibrary.VLerp` (`self.K2_GetActorLocation` (`self.point-0`)) (`self.K2_GetActorLocation` (`self.point-1`)) _alphavalue) false false)
      (if (>= _alphavalue 0.99)
        (`SceneComponent.SetWorldScale3D` _paperflipbook (1.0 1.0 1.0))
        (elif (<= _alphavalue 0.05)
          (`SceneComponent.SetWorldScale3D` _paperflipbook (-1.0 1.0 1.0)))))
    (:`Finished`
      (`KismetSystemLibrary.PrintString` "Loop End")
      (`PaperFlipbookComponent.SetFlipbook` (`self.PaperFlipbook`) "/Game/Marionic/Sprites/Enemy/fly_dead.fly_dead")
      (`ActorComponent.Deactivate` (`self.Box`))
      (`KismetSystemLibrary.Delay` 1.0)
      (`self.K2_DestroyActor`))))

(event `self.Box.OnComponentBeginOverlap`
  (params (OtherActor :type "Actor Object Reference") (OtherComp :type "PrimitiveComponent Object Reference") (OtherBodyIndex :type Integer) (bFromSweep :type Boolean) (SweepResult :type "HitResult Structure (by ref)"))
  (bind _asmarionic (cast `/Game/Marionic/Blueprints/Marionic` OtherActor))
  (`/Game/Marionic/Blueprints/Marionic.Damage System` _asmarionic (`self.damage`)))

(fn `UserConstructionScript`)